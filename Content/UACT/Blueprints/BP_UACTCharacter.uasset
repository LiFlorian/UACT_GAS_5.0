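; Player character Blueprint that adds foot IK for uneven ground and triggers attack abilities.
; Each tick it line-traces under both feet, sends the lower offset to ABP_UACT as mesh offset, and passes the height difference as the other foot's adjustment.
; Capsule half height follows half the mesh offset.
; Attack and SkillF presses activate GA_Attack and GA_DashAttack through the Ability System.
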(event EventBeginPlay
  (Utilities|FlowControl|Sequence
    (:then_0
      (bind _asabp_uact (Utilities|Casting|CastToABP_UACT (Components|SkeletalMesh|GetAnimInstance (Variables|Character|GetMesh))))
      (Variables|Default|SetAnimBP _asabp_uact))
    (:then_1
      (Variables|Default|SetCapsuleHalfHeight (Variables|/Script/Engine.CapsuleComponent|GetCapsuleHalfHeight (Variables|Default|GetCapsuleComponent))))))

(event EventTick
  (params (DeltaSeconds :type Float%20%28single-precision%29))
  (bind _animbp (Variables|Default|GetAnimBP))
  (bind _animbp_2 (Variables|Default|GetAnimBP))
  (bind _distance (CallFunction|IKLineTrace "Foot_L" 5e+01))
  (bind _distance_2 (CallFunction|IKLineTrace "Foot_R" 5e+01))
  (if (< _distance_2 _distance)
    (Variables|/Game/UACT/Animations/ABP_UACT.ABP_UACT_C|SetMeshOffset _animbp_2 _distance_2)
    (Variables|/Game/UACT/Animations/ABP_UACT.ABP_UACT_C|SetFoot_L_Adjust _animbp_2 (Math|Float|Absolute(Float) (- _distance_2 _distance)))
    (Variables|/Game/UACT/Animations/ABP_UACT.ABP_UACT_C|SetFoot_R_Adjust _animbp_2 0.0)
    (else
      (Variables|/Game/UACT/Animations/ABP_UACT.ABP_UACT_C|SetMeshOffset _animbp _distance)
      (Variables|/Game/UACT/Animations/ABP_UACT.ABP_UACT_C|SetFoot_L_Adjust _animbp 0.0)
      (Variables|/Game/UACT/Animations/ABP_UACT.ABP_UACT_C|SetFoot_R_Adjust _animbp (* (Math|Float|Absolute(Float) (- _distance_2 _distance)) -1.0))))
  (Components|Capsule|SetCapsuleHalfHeight (Variables|Default|GetCapsuleComponent) (+ (Variables|Default|GetCapsuleHalfHeight) (* (Variables|/Game/UACT/Animations/ABP_UACT.ABP_UACT_C|GetMeshOffset (Variables|Default|GetAnimBP)) 0.5)) true))

(event EventOnAttackPressed
  (Abilities|TryActivateAbilitybyClass (Variables|Default|GetAbilitySystem) "/Game/UACT/Skill/GA/GA_Attack.GA_Attack_C" true))

(event EventOnSkillFPressed
  (Abilities|TryActivateAbilitybyClass (Variables|Default|GetAbilitySystem) "/Game/UACT/Skill/GA/GA_DashAttack.GA_DashAttack_C" true))

(fn ConstructionScript)

(fn IKLineTrace
  (params (BoneName :type Name) (TraceLength :type Float%20%28double-precision%29))
  (bind _mesh (Variables|Character|GetMesh))
  (bind _returnvalue (Transformation|GetSocketLocation _mesh BoneName))
  (bind _returnvalue_2 (Transformation|GetWorldLocation _mesh))
  (bind _returnvalue_3 (Math|Vector|MakeVector (.x _returnvalue) (.y _returnvalue) (.z _returnvalue_2)))
  (bind (_outhit _returnvalue_4) (Collision|LineTraceByChannel (+ _returnvalue_3 (Math|Vector|MakeVector 0.0 0.0 (Variables|Default|GetCapsuleHalfHeight))) (- _returnvalue_3 (Math|Vector|MakeVector 0.0 0.0 TraceLength)) "TraceTypeQuery1" false 0 "None"))
  (return (Math|Float|SelectFloat (- (Variables|Default|GetCapsuleHalfHeight) (.Distance (Collision|BreakHitResult _outhit))) 0.0 _returnvalue_4)))